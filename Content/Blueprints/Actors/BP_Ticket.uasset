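; BP_Ticket is a ticket actor that displays its travel destination as text.
; On BeginPlay it switches on the Destination enum and sets its TextRender to a hardcoded Latin-script name for Moscow or Mozhaysk.
; The overlap and tick events are disabled stubs, and the construction script only calls its parent.
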(event `self.ReceiveBeginPlay`
  (bind _textrender (`self.TextRender`))
  (`parent.ReceiveBeginPlay`)
  (switch `string` (`self.Destination`)
    (:`Москва`
      (`TextRenderComponent.K2_SetText` _textrender "Moscow"))
    (:`Можайск`
      (`TextRenderComponent.K2_SetText` _textrender "Mogaiska"))))

(fn `UserConstructionScript`
  (`parent.UserConstructionScript`))