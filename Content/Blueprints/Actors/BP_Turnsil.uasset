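; BP_Turnsil is a ticket turnstile that opens its two doors when an overlapping BP_Ticket matches its Destination.
; Two trigger spheres run the same check, turning Niagara lights green on a match or red otherwise.
; One second after overlap ends, the lights turn blue and the doors snap back to positions cached at BeginPlay.
; The SpecialFuntion override switches the lights and sphere collision on or off.
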(event `CloseDoors`
  (`SceneComponent.K2_SetRelativeLocation` (`self.RightDoor`) (`self.RightDoorLocation`) false true)
  (`SceneComponent.K2_SetRelativeLocation` (`self.LeftDoor`) (`self.LeftDoorLocation`) false true))

(event `OpenDoors`
  (`SceneComponent.K2_AddRelativeLocation` (`self.RightDoor`) (50.0 0.0 0.0) false true)
  (`SceneComponent.K2_AddRelativeLocation` (`self.LeftDoor`) (50.0 0.0 0.0) false true))

(event `self.ReceiveBeginPlay`
  (`parent.ReceiveBeginPlay`)
  (set `self.RightDoorLocation` (`SceneComponent.RelativeLocation` (`self.RightDoor`)))
  (set `self.LeftDoorLocation` (`SceneComponent.RelativeLocation` (`self.LeftDoor`))))

(event `SwitchColors`
  (params (MainColor :type "LinearColor Structure") (SecColor :type "LinearColor Structure"))
  (bind _fx_atmlights2 (`self.FX_ATMLights2`))
  (`FXSystemComponent.SetColorParameter` _fx_atmlights2 "User.MainColor" MainColor)
  (`FXSystemComponent.SetColorParameter` (`self.FX_ATMLights1`) "User.MainColor" MainColor)
  (`FXSystemComponent.SetColorParameter` (`self.FX_ATMLights`) "User.MainColor" MainColor)
  (`FXSystemComponent.SetColorParameter` (`self.FX_ATMLights3`) "User.MainColor" MainColor)
  (`FXSystemComponent.SetColorParameter` _fx_atmlights2 "User.SecondaryColor" SecColor)
  (`FXSystemComponent.SetColorParameter` (`self.FX_ATMLights1`) "User.SecondaryColor" SecColor)
  (`FXSystemComponent.SetColorParameter` (`self.FX_ATMLights`) "User.SecondaryColor" SecColor)
  (`FXSystemComponent.SetColorParameter` (`self.FX_ATMLights3`) "User.SecondaryColor" SecColor))

(event `self.Sphere.OnComponentBeginOverlap`
  (params (OverlappedComponent :type "PrimitiveComponent Object Reference") (OtherActor :type "Actor Object Reference") (OtherComp :type "PrimitiveComponent Object Reference") (OtherBodyIndex :type Integer) (bFromSweep :type Boolean) (SweepResult :type "HitResult Structure (by ref)"))
  (bind _asbp_ticket (cast `/Game/Blueprints/Actors/BP_Ticket` OtherActor))
  (if (`KismetStringLibrary.EqualEqual_StrStr` (`/Game/Blueprints/Actors/BP_Ticket.Destination` _asbp_ticket) (`self.Destination`))
    (`self.OpenDoors`)
    (`self.SwitchColors` (struct :`G` 30.0 :`B` 2.0 :`A` 1.0) (struct :`G` 1.0 :`B` 0.2 :`A` 1.0) :!label _label)
    (else
      (`self.SwitchColors` (struct :`R` 30.0 :`A` 1.0) (struct :`R` 1.0 :`A` 1.0) :!label _label_2))))

(event `self.Sphere1.OnComponentBeginOverlap`
  (params (OverlappedComponent :type "PrimitiveComponent Object Reference") (OtherActor :type "Actor Object Reference") (OtherComp :type "PrimitiveComponent Object Reference") (OtherBodyIndex :type Integer) (bFromSweep :type Boolean) (SweepResult :type "HitResult Structure (by ref)"))
  (bind _asbp_ticket (cast `/Game/Blueprints/Actors/BP_Ticket` OtherActor))
  (if (`KismetStringLibrary.EqualEqual_StrStr` (`/Game/Blueprints/Actors/BP_Ticket.Destination` _asbp_ticket) (`self.Destination`))
    (`self.OpenDoors`)
    (goto _label)
    (else
      (goto _label_2))))

(event `self.Sphere.OnComponentEndOverlap`
  (params (OverlappedComponent :type "PrimitiveComponent Object Reference") (OtherActor :type "Actor Object Reference") (OtherComp :type "PrimitiveComponent Object Reference") (OtherBodyIndex :type Integer))
  (`KismetSystemLibrary.Delay` 1.0)
  (`self.SwitchColors` (struct :`B` 30.0 :`A` 1.0) (struct :`G` 0.2 :`B` 1.0 :`A` 1.0) :!label _label_3)
  (`self.CloseDoors`))

(event `self.Sphere1.OnComponentEndOverlap`
  (params (OverlappedComponent :type "PrimitiveComponent Object Reference") (OtherActor :type "Actor Object Reference") (OtherComp :type "PrimitiveComponent Object Reference") (OtherBodyIndex :type Integer))
  (`KismetSystemLibrary.Delay` 1.0)
  (goto _label_3))

(fn `SpecialFuntion`
  (params (Active :type Boolean))
  (`parent.SpecialFuntion` Active)
  (`ActorComponent.SetActive` (`self.FX_ATMLights1`) Active false)
  (`ActorComponent.SetActive` (`self.FX_ATMLights`) Active false)
  (`ActorComponent.SetActive` (`self.FX_ATMLights2`) Active false)
  (`ActorComponent.SetActive` (`self.FX_ATMLights3`) Active false)
  (`PrimitiveComponent.SetCollisionEnabled` (`self.Sphere`) (select `bool` Active :`false` "NoCollision" :`true` "QueryOnly" :!type "ECollisionEnabled Enum"))
  (`PrimitiveComponent.SetCollisionEnabled` (`self.Sphere1`) (select `bool` Active :`false` "NoCollision" :`true` "QueryOnly" :!type "ECollisionEnabled Enum")))

(fn `UserConstructionScript`
  (`parent.UserConstructionScript`))