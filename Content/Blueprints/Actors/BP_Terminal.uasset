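; BP_Terminal is a payment terminal actor that issues a destination ticket when a card is presented.
; It hands its reference to its UI_Terminal widget and toggles the card-detection sphere and ATM light effects between waiting and idle states.
; When a BP_Card overlaps the active sphere, it spawns a BP_Ticket at the mesh's Ticket socket with the widget's chosen destination, then fires OnPayed.
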(event `self.ReceiveBeginPlay`
  (bind _asui_terminal (cast `/Game/UI_Terminal` (`WidgetComponent.GetUserWidgetObject` (`self.Widget`))))
  (set `/Game/UI_Terminal.TerminalRef` self _asui_terminal)
  (`PrimitiveComponent.SetCollisionEnabled` (`self.Sphere`) "NoCollision")
  (add `self.OnPayed` (`|CreateDelegate` :!event `ResetToIdle`)))

(event `SpawnTicket`
  (params (Destination :type String))
  (`|SpawnActorFromClass` "/Game/Blueprints/Actors/BP_Ticket.BP_Ticket_C" (`SceneComponent.GetSocketTransform` (`self.StaticMesh`) "Ticket" "RTS_World") "Undefined" "OverrideRootScale" null Destination null))

(event `WaitnigForCard`
  (`PrimitiveComponent.SetCollisionEnabled` (`self.Sphere`) "QueryOnly")
  (`ActorComponent.SetActive` (`self.FX_ATMLights1`) true false)
  (`ActorComponent.SetActive` (`self.FX_ATMLights`) true false))

(event `ResetToIdle`
  (`PrimitiveComponent.SetCollisionEnabled` (`self.Sphere`) "NoCollision")
  (`ActorComponent.SetActive` (`self.FX_ATMLights1`) false false)
  (`ActorComponent.SetActive` (`self.FX_ATMLights`) false false))

(event `self.Sphere.OnComponentBeginOverlap`
  (params (OverlappedComponent :type "PrimitiveComponent Object Reference") (OtherActor :type "Actor Object Reference") (OtherComp :type "PrimitiveComponent Object Reference") (OtherBodyIndex :type Integer) (bFromSweep :type Boolean) (SweepResult :type "HitResult Structure (by ref)"))
  (cast `/Game/Blueprints/Actors/BP_Card` OtherActor)
  (`self.SpawnTicket` (`/Game/UI_Terminal.TicketDestination` (cast `/Game/UI_Terminal` (`WidgetComponent.GetUserWidgetObject` (`self.Widget`)) :!pure true)))
  (`self.OnPayed`))

(fn `UserConstructionScript`)