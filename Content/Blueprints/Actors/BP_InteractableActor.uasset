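; Base interactable actor that can be highlighted through custom depth and notifies the player's pawn on Interact when TakeAway is set.
; BeginPlay picks the static mesh, or else the skeletal mesh, as the active component, then gives it query-only Visibility-blocking collision and a stencil value.
; Activate toggles that mesh's custom depth rendering.
; The empty SpecialFuntion hook runs only on the static mesh path.
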(event `self.ReceiveBeginPlay`
  (`self.DefineActiveComponent`)
  (`self.SetCollisions`)
  (`self.SetStencilValue`))

(event `/Game/Blueprints/Interfaces/BPI_InteractionItems.Interact`
  (if (`self.TakeAway`)
    (message `/Game/Blueprints/Interfaces/BPI_InteractionItems.Interact` (`Controller.K2_GetPawn` (`GameplayStatics.GetPlayerController` 0)))))

(fn `Activate`
  (params (SetActive :type Boolean))
  (switch `/Game/Blueprints/Enums/EActiveComponent` (`self.ActiveComponent`)
    (:`NewEnumerator0`
      (`PrimitiveComponent.SetRenderCustomDepth` (`self.StaticMesh`) SetActive)
      (`self.SpecialFuntion` SetActive))
    (:`NewEnumerator1`
      (`PrimitiveComponent.SetRenderCustomDepth` (`self.SkeletalMesh`) SetActive))))

(fn `DefineActiveComponent`
  (`|ExecutionSequence`
    (:`then_0`
      (set `self.ActiveComponent` (select `bool` (`KismetSystemLibrary.IsValid` (`StaticMeshComponent.StaticMesh` (`self.StaticMesh`))) :`false` "NewEnumerator2" :`true` "NewEnumerator0" :!type "/Game/Blueprints/Enums/EActiveComponent Enum")))
    (:`then_1`
      (if (`|EnumEquality` (`self.ActiveComponent`) "NewEnumerator2")
        (set `self.ActiveComponent` (select `bool` (`KismetSystemLibrary.IsValid` (`SkinnedMeshComponent.SkeletalMesh` (`self.SkeletalMesh`))) :`false` "NewEnumerator2" :`true` "NewEnumerator1" :!type "/Game/Blueprints/Enums/EActiveComponent Enum"))))))

(fn `SetCollisions`
  (bind _staticmesh (`self.StaticMesh`))
  (bind _skeletalmesh (`self.SkeletalMesh`))
  (switch `/Game/Blueprints/Enums/EActiveComponent` (`self.ActiveComponent`)
    (:`NewEnumerator0`
      (`PrimitiveComponent.SetCollisionEnabled` _staticmesh "QueryOnly")
      (`PrimitiveComponent.SetCollisionResponseToChannel` _staticmesh "ECC_Visibility" "ECR_Block")
      (`PrimitiveComponent.SetCollisionEnabled` (`self.SkeletalMesh`) "NoCollision"))
    (:`NewEnumerator1`
      (`PrimitiveComponent.SetCollisionEnabled` _skeletalmesh "QueryOnly")
      (`PrimitiveComponent.SetCollisionResponseToChannel` _skeletalmesh "ECC_Visibility" "ECR_Block")
      (`PrimitiveComponent.SetCollisionEnabled` (`self.StaticMesh`) "NoCollision"))))

(fn `SetStencilValue`
  (locals (LocalSMStancil :type Integer) (LocalSKStancil :type Integer))
  (bind _staticmesh (`self.StaticMesh`))
  (bind _skeletalmesh (`self.SkeletalMesh`))
  (bind _activecomponent (`self.ActiveComponent`))
  (set `local.LocalSMStancil` (select `/Game/Blueprints/Enums/EActiveComponent` _activecomponent :`NewEnumerator0` 1))
  (set `local.LocalSKStancil` (select `/Game/Blueprints/Enums/EActiveComponent` _activecomponent :`NewEnumerator1` 1))
  (`PrimitiveComponent.SetCustomDepthStencilValue` _staticmesh (`local.LocalSMStancil`))
  (`PrimitiveComponent.SetRenderCustomDepth` _staticmesh false)
  (`PrimitiveComponent.SetCustomDepthStencilValue` _skeletalmesh (`local.LocalSKStancil`))
  (`PrimitiveComponent.SetRenderCustomDepth` _skeletalmesh false))

(fn `SpecialFuntion`
  (params (Active :type Boolean)))

(fn `UserConstructionScript`)